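; BP_XR_Player is the XR player pawn with a body mesh that scales to the player's estimated height and hideable body and hand sections.
; When locally controlled, it converts both hands' tracking rotations and sends them with positions, height and movement speed to BP_XR_PlayerState.
; Auto height jumps up to higher camera positions and eases down slowly, driving mesh scale, vertical offset and floor height.
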(event EventBeginPlay
  (bind _hide_hands (Variables|Default|GetHide%20Hands))
  (bind _returnvalue (not _hide_hands))
  ;[1 1 1] Init
  (Variables|Default|SetLocation (* (Transformation|GetWorldLocation (Variables|Default|GetParentRelativeAttachment)) "1.000000,1.000000,0.000000"))
  (Class|SkinnedMeshComponent|ShowMaterialSection (Variables|Character|GetMesh) 2 0 (not (Variables|Default|GetHide%20Body)))
  (Class|SkinnedMeshComponent|ShowMaterialSection (Variables|Character|GetMesh) 0 0 _returnvalue)
  (Class|SkinnedMeshComponent|ShowMaterialSection (Variables|Character|GetMesh) 1 0 _returnvalue))

(event EventTick
  (params (DeltaSeconds :type Float%20%28single-precision%29))
  (bind _vrreplicatedcamera (Variables|Default|GetVRReplicatedCamera))
  (bind _mesh (Variables|Character|GetMesh))
  (bind _parentrelativeattachment (Variables|Default|GetParentRelativeAttachment))
  (bind _returnvalue (Transformation|GetWorldLocation _parentrelativeattachment))
  (bind _returnvalue_2 (Transformation|GetWorldRotation _vrreplicatedcamera))
  (bind _returnvalue_3 (Transformation|GetWorldLocation _vrreplicatedcamera))
  (bind _returnvalue_4 (Math|Vector|GetForwardVector _returnvalue_2))
  (bind _returnvalue_5 (* _returnvalue "1.000000,1.000000,0.000000"))
  (bind _returnvalue_6 (* _returnvalue_4 -1e+01))
  (bind _returnvalue_7 (+ _returnvalue_3 _returnvalue_6))
  (Utilities|FlowControl|Sequence
    (:then_0
      ;[1 1 1] Hand Tracking
      (if (Pawn|IsLocallyControlled)
        (bind _asbp_xr_player_state (Utilities|Casting|CastToBP_XR_PlayerState (Variables|Default|GetPlayerState)))
        (bind _motioncontrollerdata (Class|HeadMountedDisplayFunctionLibrary|GetMotionControllerData self "Left"))
        (bind (_tracked _rotations _location) (CallFunction|ProcessTracking _motioncontrollerdata false))
        (bind _motioncontrollerdata_2 (Class|HeadMountedDisplayFunctionLibrary|GetMotionControllerData self "Right"))
        (bind (_tracked_2 _rotations_2 _location_2) (CallFunction|ProcessTracking _motioncontrollerdata_2 true))
        (Default|UpdateHandState _asbp_xr_player_state (Utilities|Struct|MakeS_XR_HandState _tracked _tracked_2 _rotations _rotations_2 _location _location_2 (+ (- 165.0 (.Z (Math|Vector|BreakVector _returnvalue))) (Variables|Default|GetFloorHeight)) (/ (Math|Vector|VectorLength (- _returnvalue_5 (Variables|Default|GetLocation))) DeltaSeconds)))
        (Variables|Default|SetLocation _returnvalue_5)))
    (:then_1
      ;[1 1 1] Auto Height
      (if (> (.z _returnvalue_7) (Variables|Default|GetMeanHeight))
        (Variables|Default|SetMeanHeight (.z _returnvalue_7))
        (else
          (bind _output_get (Variables|Default|SetMeanHeight (Math|Float|Lerp (Variables|Default|GetMeanHeight) (.z _returnvalue_7) 0.005)))))
      (Transformation|SetRelativeScale3D _mesh (Math|Conversions|ToVector(Float) (/ _output_get 1.7e+02)))
      (Transformation|SetRelativeLocation _mesh (Math|Vector|MakeVector -5.0 0.0 (* _output_get -1.0)) false true)
      (Variables|Default|SetFloorHeight (- _output_get 1.7e+02)))))

(fn ConstructionScript)

(fn ProcessTracking
  (params (Data :type XR%20Motion%20Controller%20Data%20Structure%20%28by%20ref%29) (Handedness :type Boolean))
  (bind (_bvalid _devicename _applicationinstanceid _devicevisualtype _handindex _trackingstatus _gripposition _griprotation _aimposition _aimrotation _palmposition _palmrotation _handkeypositions _handkeyrotations) (Utilities|Struct|BreakXRMotionControllerData Data))
  (Utilities|FlowControl|Sequence
    (:then_0
      (if _bvalid
        (for _array_element _handkeyrotations
          (if Handedness
            (Utilities|Array|Add (LocalVariables|GetRotations_Temp) (Math|Rotator|MakeRotator (+ (* (.Roll (Math|Rotator|BreakRotator (Class|KismetMathLibrary|QuatRotator _array_element))) -1.0) 9e+01) (* (.Pitch (Math|Rotator|BreakRotator (Class|KismetMathLibrary|QuatRotator _array_element))) -1.0) (+ (.Yaw (Math|Rotator|BreakRotator (Class|KismetMathLibrary|QuatRotator _array_element))) 1.8e+02)))
            (else
              (Utilities|Array|Add (LocalVariables|GetRotations_Temp) (Math|Rotator|MakeRotator (+ (* (.Roll (Math|Rotator|BreakRotator (Class|KismetMathLibrary|QuatRotator _array_element))) 1.0) 9e+01) (+ (* (.Pitch (Math|Rotator|BreakRotator (Class|KismetMathLibrary|QuatRotator _array_element))) -1.0) 1.8e+02) (+ (.Yaw (Math|Rotator|BreakRotator (Class|KismetMathLibrary|QuatRotator _array_element))) 1.8e+02))))))
        (LocalVariables|SetLocation_Temp (Utilities|Array|Get(acopy) _handkeypositions 1))))
    (:then_1
      (return _bvalid (LocalVariables|GetRotations_Temp) (LocalVariables|GetLocation_Temp)))))

(fn OnRepHideBody
  (Class|SkinnedMeshComponent|ShowMaterialSection (Variables|Character|GetMesh) 2 0 (not (Variables|Default|GetHide%20Body))))

(fn OnRepHideHands)

(fn OnRepHideUntrackedHand)

(fn OnRepHT)